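; BP_TestCharacter is a minimal first-person test character for trying out physics interaction abilities on interactables.
; Enhanced Input drives movement, look and jump, while hardcoded number keys trigger grab, drop, poke and throw, mostly through the BPCharacterPhysicsAbilities component.
; Grab and poke use tolerant line traces from the Camera; grabbed objects attach to it and ease into a held position.
; Throw responds to both key press and release.
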(event `Key|One`
  (params (Key :type "Key Structure"))
  ;[1 1 1] Grab Nicer
  (:`Pressed`
    (bind _outhit (`CommonFunctions.LineTraceSingleWithToleranceByReference` :`ComponentReference` (`self.Camera`) :`TraceLength` 500.0 :`DrawTime` 0.0 :`DebugThickness` 1.0 :`TraceColor` (struct :`R` 255 :`A` 255) :`TraceHitColor` (struct :`G` 255 :`A` 255)))
    (bind _returnvalue (`CharacterPhysicsAbilities.GrabInteractable` (`self.BP_CharacterPhysicsAbilities`) _outhit (`self.Camera`) true))
    (`KismetSystemLibrary.MoveComponentTo` _returnvalue (100.0 0.0 -50.0) (struct) true true 0.2 true)))

(event `Key|Four`
  (params (Key :type "Key Structure"))
  ;[1 1 1] Throw Nicer
  (:`Pressed`
    (`CharacterPhysicsAbilities.ThrowInteractable` (`self.BP_CharacterPhysicsAbilities`) -1.0 :!label _label))
  (:`Released`
    (goto _label :!via `Released`)))

(event `self.ReceiveBeginPlay`
  ;[1 1 1] Input, Movement, Look, Jump
  (`EnhancedInputSubsystemInterface.AddMappingContext` (pcsubsystem `EnhancedInputLocalPlayerSubsystem` (`GameplayStatics.GetPlayerController` 0)) "/PhysicsAbilities/MinimalCharacter/Inputs/IMC_MainContexMapping.IMC_MainContexMapping" 0 (struct)))

(event `EnhancedInput|/PhysicsAbilities/MinimalCharacter/Inputs/InputActions/IA_LookUp`
  (params (ActionValue :type "Float (double-precision)") (ElapsedSeconds :type "Float (double-precision)") (TriggeredSeconds :type "Float (double-precision)") (InputAction :type "InputAction Object Reference" :default "/PhysicsAbilities/MinimalCharacter/Inputs/InputActions/IA_LookUp.IA_LookUp"))
  ;[1 1 1] Input, Movement, Look, Jump
  (:`Triggered`
    (`self.AddControllerPitchInput` ActionValue)))

(event `EnhancedInput|/PhysicsAbilities/MinimalCharacter/Inputs/InputActions/IA_MoveForward`
  (params (ActionValue :type "Float (double-precision)") (ElapsedSeconds :type "Float (double-precision)") (TriggeredSeconds :type "Float (double-precision)") (InputAction :type "InputAction Object Reference" :default "/PhysicsAbilities/MinimalCharacter/Inputs/InputActions/IA_MoveForward.IA_MoveForward"))
  ;[1 1 1] Input, Movement, Look, Jump
  (:`Triggered`
    (`self.AddMovementInput` (`self.GetActorForwardVector`) ActionValue)))

(event `EnhancedInput|/PhysicsAbilities/MinimalCharacter/Inputs/InputActions/IA_MoveRight`
  (params (ActionValue :type "Float (double-precision)") (ElapsedSeconds :type "Float (double-precision)") (TriggeredSeconds :type "Float (double-precision)") (InputAction :type "InputAction Object Reference" :default "/PhysicsAbilities/MinimalCharacter/Inputs/InputActions/IA_MoveRight.IA_MoveRight"))
  ;[1 1 1] Input, Movement, Look, Jump
  (:`Triggered`
    (`self.AddMovementInput` (`self.GetActorRightVector`) ActionValue)))

(event `EnhancedInput|/PhysicsAbilities/MinimalCharacter/Inputs/InputActions/IA_LookRight`
  (params (ActionValue :type "Float (double-precision)") (ElapsedSeconds :type "Float (double-precision)") (TriggeredSeconds :type "Float (double-precision)") (InputAction :type "InputAction Object Reference" :default "/PhysicsAbilities/MinimalCharacter/Inputs/InputActions/IA_LookRight.IA_LookRight"))
  ;[1 1 1] Input, Movement, Look, Jump
  (:`Triggered`
    (`self.AddControllerYawInput` ActionValue)))

(event `Key|Three`
  (params (Key :type "Key Structure"))
  ;[1 1 1] Poke Nicer
  (:`Pressed`
    (bind _outhit (`CommonFunctions.LineTraceSingleWithToleranceByReference` :`ComponentReference` (`self.Camera`) :`TraceLength` 500.0 :`DrawTime` 0.0 :`DebugThickness` 1.0 :`TraceColor` (struct :`R` 255 :`A` 255) :`TraceHitColor` (struct :`G` 255 :`A` 255)))
    (`CharacterPhysicsAbilities.PokeInteractable` (`self.BP_CharacterPhysicsAbilities`) _outhit (`SceneComponent.GetForwardVector` (`self.Camera`)) -1.0)))

(event `Key|Two`
  (params (Key :type "Key Structure"))
  ;[1 1 1] Drop Nicer
  (:`Pressed`
    (`CharacterPhysicsAbilities.DropInteractable` (`self.BP_CharacterPhysicsAbilities`))))

(event `EnhancedInput|/PhysicsAbilities/MinimalCharacter/Inputs/InputActions/IA_Jump`
  (params (ActionValue :type Boolean) (ElapsedSeconds :type "Float (double-precision)") (TriggeredSeconds :type "Float (double-precision)") (InputAction :type "InputAction Object Reference" :default "/PhysicsAbilities/MinimalCharacter/Inputs/InputActions/IA_Jump.IA_Jump"))
  ;[1 1 1] Input, Movement, Look, Jump
  (:`Triggered`
    (if ActionValue
      (`self.Jump`)
      (else
        (`self.StopJumping`)))))

(fn `UserConstructionScript`)