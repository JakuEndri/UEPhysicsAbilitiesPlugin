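; Test prop cube with a configurable mass, used to exercise grab, drop, throw and poke interactions.
; The construction script overrides the static mesh mass with the Mass value and shows it on four text renders.
; Interaction checks always return true, and both they and the interaction events only print their names for debugging.
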(event `self.Grabb`
  (params (Interactor :type "Object Object Reference") (Hit :type "HitResult Structure (by ref)"))
  (`KismetSystemLibrary.PrintString` "Grabbed"))

(event `self.Throw`
  (params (Interactor :type "Object Object Reference"))
  (`KismetSystemLibrary.PrintString` "Throw"))

(event `self.StartThrowing`
  (params (Interactor :type "Object Object Reference"))
  (`KismetSystemLibrary.PrintString` "StartThrowing"))

(event `self.Poke`
  (params (Interactor :type "Object Object Reference") (Hit :type "HitResult Structure (by ref)"))
  (`KismetSystemLibrary.PrintString` "Poke"))

(event `self.Drop`
  (params (Interactor :type "Object Object Reference") (GrabbedBone :type Name))
  (`KismetSystemLibrary.PrintString` "Drop"))

(fn `CanBeDropped`
  (params (Interactor :type "Object Object Reference"))
  (returns (ReturnValue :type Boolean))
  (`KismetSystemLibrary.PrintString` "CanBeDropped")
  (return true))

(fn `CanBeGrabbed`
  (params (Interactor :type "Object Object Reference") (Hit :type "HitResult Structure (by ref)"))
  (returns (ReturnValue :type Boolean))
  (`KismetSystemLibrary.PrintString` "CanBeGrabbed")
  (return true))

(fn `CanBePoked`
  (params (Interactor :type "Object Object Reference") (Hit :type "HitResult Structure (by ref)") (Direction :type "Vector Structure (by ref)"))
  (returns (ReturnValue :type Boolean))
  (`KismetSystemLibrary.PrintString` "CanBePoked")
  (return true))

(fn `CanBeThrown`
  (params (Interactor :type "Object Object Reference"))
  (returns (ReturnValue :type Boolean))
  (`KismetSystemLibrary.PrintString` "CanBeThrown")
  (return true))

(fn `CanStartThrowing`
  (params (Interactor :type "Object Object Reference"))
  (returns (ReturnValue :type Boolean))
  (`KismetSystemLibrary.PrintString` "CanStartThrowing")
  (return true))

(fn `SetMass`
  (params (Mass :type "Float (double-precision)"))
  (bind _returnvalue (`KismetTextLibrary.Conv_DoubleToText` Mass "HalfToEven"))
  (`PrimitiveComponent.SetMassOverrideInKg` (`self.StaticMesh`) "None" Mass true)
  (`TextRenderComponent.K2_SetText` (`self.TextRender`) _returnvalue)
  (`TextRenderComponent.K2_SetText` (`self.TextRender1`) _returnvalue)
  (`TextRenderComponent.K2_SetText` (`self.TextRender2`) _returnvalue)
  (`TextRenderComponent.K2_SetText` (`self.TextRender3`) _returnvalue))

(fn `UserConstructionScript`
  (`self.SetMass` (`self.Mass`)))